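; BP_MegaCharacter is a character Blueprint with throw and pick-up animations plus debug-style keys for slow motion and noise.
; Enhanced Input actions IA_Throw and IA_Interact only play sped-up montages on the mesh.
; CapsLock toggles global time dilation through a FlipFlop, while G reports a wide-range AI noise event and prints confirmation.
; Logic to snap BP_Torch to the mesh's TorchSocket exists but is unconnected and never runs.
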(event Input|EnhancedActionEvents|EnhancedInputActionIA_Throw
  (params (ActionValue :type Boolean) (ElapsedSeconds :type Float%20%28double-precision%29) (TriggeredSeconds :type Float%20%28double-precision%29) (InputAction :type Input%20Action%20Object%20Reference :default "/Game/Inputs/Actions/IA_Throw.IA_Throw"))
  (:Started
    (Animation|Montage|PlayMontage (Variables|Character|GetMesh) "/Game/Character/Animations/AM_Throw_.AM_Throw_" 1.5)))

(event Input|EnhancedActionEvents|EnhancedInputActionIA_Interact
  (params (ActionValue :type Boolean) (ElapsedSeconds :type Float%20%28double-precision%29) (TriggeredSeconds :type Float%20%28double-precision%29) (InputAction :type Input%20Action%20Object%20Reference :default "/Game/Inputs/Actions/IA_Interact.IA_Interact"))
  (:Started
    (Animation|Montage|PlayMontage (Variables|Character|GetMesh) "/Game/Character/Animations/AM_Pick.AM_Pick" 2.0)))

(event Collision|EventActorBeginOverlap
  (params (OtherActor :type Actor%20Object%20Reference)))

(event Input|KeyboardEvents|CapsLock
  (params (Key :type Key%20Structure :default "None"))
  ;[1 1 1] Slomotion
  (:Pressed
    (Utilities|FlowControl|FlipFlop
      (:A
        (Utilities|Time|SetGlobalTimeDilation 0.2))
      (:B
        (Utilities|Time|SetGlobalTimeDilation 1.0)))))

(event Input|KeyboardEvents|G
  (params (Key :type Key%20Structure :default "None"))
  (:Pressed
    (Utilities|FlowControl|Sequence
      (:then_0
        (Class|AISenseHearing|ReportNoiseEvent (Transformation|GetActorLocation) 1.0 self 5e+03 "None")
        (Development|PrintString "Noise Created" true true "(R=0.000000,G=0.660000,B=1.000000,A=1.000000)" 1.0)))))

(fn ConstructionScript)